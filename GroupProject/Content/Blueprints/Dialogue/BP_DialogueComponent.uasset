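; Dialogue component that runs branching conversations from data table rows in a WB_Dialogue widget.
; Interact opens the widget with game-and-UI input, advances through each row's next row and table, then closes after an end-flagged row.
; Open-ended rows spawn WB_Options entries on opening or option selection, but not when Interact advances.
; OptionSelected jumps to the chosen row, while LeaveDialogue closes the widget and restores game-only input.
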(event `Option Selected`
  (params (RowName :type Name) (DataTable :type "DataTable Object Reference"))
  (bind _dialoguewidget (`self.DialogueWidget`))
  ; Dialogue Options
  (bind _returnvalue (`|GetDataTableRow` DataTable RowName)
    (:`then`
      (`PanelWidget.ClearChildren` (`/Game/Blueprints/Dialogue/WB_Dialogue.OptionsScrollBox` _dialoguewidget))
      (bind (_dialogue _nextrow _datatable _enddialogue _openendeddialogue_ _openendeddialogueoptions) (break `/Game/Blueprints/Dialogue/Dialouge_Structure` _returnvalue))
      (`/Game/Blueprints/Dialogue/WB_Dialogue.Update Dialogue` _dialoguewidget _dialogue)
      (set `self.Row Name` _nextrow)
      (set `self.Data Table` _datatable)
      (set `self.EndDialouge` _enddialogue)
      ; Repeat Adding these to Add more Options/Prompts/Responses
      (if _openendeddialogue_
        (for _array_element _openendeddialogueoptions
          (bind (_optionname _row _datatable_2) (break `/Game/Blueprints/Dialogue/OptionsDialogue_Structure` _array_element))
          (bind _returnvalue_2 (`|CreateWidget` "/Game/Blueprints/Dialogue/WB_Options.WB_Options_C" null (`KismetTextLibrary.Conv_NameToText` _optionname) self _row _datatable_2))
          (`PanelWidget.AddChild` (`/Game/Blueprints/Dialogue/WB_Dialogue.OptionsScrollBox` (`self.DialogueWidget`)) _returnvalue_2))))))

(event `/Game/Blueprints/Dialogue/BP_Interact.Leave Dialogue`
  (bind _returnvalue (`GameplayStatics.GetPlayerController` 0))
  ; Dialogue
  (`/Engine/EditorBlueprintResources/StandardMacros.IsValid` (`self.DialogueWidget`)
    (:`Is Valid`
      (`Widget.RemoveFromParent` (`self.DialogueWidget`) :!label _label)
      (set `self.EndDialouge` false)
      (set `self.DialogueWidget` null)
      (`WidgetBlueprintLibrary.SetInputMode_GameOnly` _returnvalue)
      (set `PlayerController.bShowMouseCursor` false _returnvalue))))

(event `/Game/Blueprints/Dialogue/BP_Interact.Interact`
  (params (PlayerRef :type "/Game/Levels/MainLevel/Blueprints/BP_ThirdPersonCharacter Object Reference"))
  (bind _returnvalue (`GameplayStatics.GetPlayerController` 0))
  ; Dialogue
  (if (`self.EndDialouge`)
    (goto _label)
    (else
      (`/Engine/EditorBlueprintResources/StandardMacros.IsValid` (`self.DialogueWidget`)
        (:`Is Valid`
          (bind _returnvalue_2 (`|GetDataTableRow` (`self.Data Table`) (`self.Row Name`))
            (:`then`
              (bind (_dialogue _nextrow _datatable _enddialogue) (break `/Game/Blueprints/Dialogue/Dialouge_Structure` _returnvalue_2))
              (`/Game/Blueprints/Dialogue/WB_Dialogue.Update Dialogue` (`self.DialogueWidget`) _dialogue)
              (set `self.Row Name` _nextrow)
              (set `self.Data Table` _datatable)
              (set `self.EndDialouge` _enddialogue))))
        (:`Is Not Valid`
          (bind _returnvalue_3 (`|GetDataTableRow` (`self.Data Table`) (`self.Row Name`))
            (:`then`
              (bind (_dialogue_2 _nextrow_2 _datatable_2 _enddialogue_2 _openendeddialogue_ _openendeddialogueoptions) (break `/Game/Blueprints/Dialogue/Dialouge_Structure` _returnvalue_3))
              (bind _returnvalue_4 (`|CreateWidget` "/Game/Blueprints/Dialogue/WB_Dialogue.WB_Dialogue_C" null (`KismetTextLibrary.Conv_NameToText` (`self.Name`)) _dialogue_2))
              (bind _output_get (set `self.DialogueWidget` _returnvalue_4))
              (`UserWidget.AddToViewport` _output_get 0)
              (set `self.Row Name` _nextrow_2)
              (set `self.Data Table` _datatable_2)
              (set `self.EndDialouge` _enddialogue_2)
              (`WidgetBlueprintLibrary.SetInputMode_GameAndUIEx` _returnvalue null)
              (set `PlayerController.bShowMouseCursor` true _returnvalue)
              (if _openendeddialogue_
                (for _array_element _openendeddialogueoptions
                  (bind (_optionname _row _datatable_3) (break `/Game/Blueprints/Dialogue/OptionsDialogue_Structure` _array_element))
                  (bind _returnvalue_5 (`|CreateWidget` "/Game/Blueprints/Dialogue/WB_Options.WB_Options_C" null (`KismetTextLibrary.Conv_NameToText` _optionname) self _row _datatable_3))
                  (`PanelWidget.AddChild` (`/Game/Blueprints/Dialogue/WB_Dialogue.OptionsScrollBox` (`self.DialogueWidget`)) _returnvalue_5))))))))))