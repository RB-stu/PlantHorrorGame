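; Quest giver component that lets its owning actor offer a quest when the player interacts with it.
; Interact asks the player character's quest log component whether the quest in QuestData is active, calling DisplayQuest if not and printing an "Already on Quest" message otherwise.
; Both branches return the owner's display name.
; DisplayQuest is an empty stub, and BeginPlay and Tick are unused.
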(fn `Display Quest`)

(fn `Interact`
  (params (PlayerRef :type "/Game/Levels/MainLevel/Blueprints/BP_ThirdPersonCharacter Object Reference"))
  (returns (InteractionID :type String))
  (bind (_questdata_datatable _questdata_rowname) (break `DataTableRowHandle` (`self.QuestData`)))
  (bind _returnvalue (`KismetSystemLibrary.GetDisplayName` (`self.GetOwner`)))
  (if (not (`/Game/Blueprints/QuestSystem/BP_QuestLogComponent.Query Active Quest` (`/Game/ThirdPerson/Blueprints/BP_Sprite.BP_QuestLogComponent` (`/Game/Blueprints/CommonFunctionLibrary.Get My Player Character`)) _questdata_rowname))
    (`self.Display Quest`)
    (return _returnvalue)
    (else
      (`KismetSystemLibrary.PrintString` "Already on Quest")
      (return _returnvalue))))