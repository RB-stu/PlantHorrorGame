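; Interactable world object that shows an interaction hint and outline while the BP_Sprite actor is within its sphere, if CanInteract is set.
; Begin overlap creates a UI_Interact widget in the Widget component, plays its PopUp animation and applies the M_Outline overlay to the mesh.
; End overlap replays PopUp, clears CanPressE and the outline, then removes and hides the widget after a short delay.
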(event `self.Sphere.OnComponentBeginOverlap`
  (params (OverlappedComponent :type "PrimitiveComponent Object Reference") (OtherActor :type "Actor Object Reference") (OtherComp :type "PrimitiveComponent Object Reference") (OtherBodyIndex :type Integer) (bFromSweep :type Boolean) (SweepResult :type "HitResult Structure (by ref)"))
  (bind _widget (`self.Widget`))
  (cast `/Game/ThirdPerson/Blueprints/BP_Sprite` OtherActor)
  (if (`self.Can Interact`)
    (bind _returnvalue (`|CreateWidget` "/Game/Blueprints/Dialogue_Interact/UI_Interact.UI_Interact_C"))
    (bind _output_get (set `self.InteractionWidget` _returnvalue))
    (`WidgetComponent.SetWidget` _widget _output_get)
    (`SceneComponent.SetVisibility` _widget true false)
    (bind _interactionwidget (`self.InteractionWidget`)
      (:`then`
        (if (not (`self.HintVisible`))
          (`UserWidget.PlayAnimation` _interactionwidget (`/Game/Blueprints/Dialogue_Interact/UI_Interact.PopUp` _interactionwidget) 0.0 1 "Forward" 1.5 false)
          (set `self.HintVisible` true)
          (`MeshComponent.SetOverlayMaterial` (`self.StaticMesh`) "/Game/Blueprints/Dialogue_Interact/M_Outline.M_Outline")))
      (:`else`))))

(event `self.Sphere.OnComponentEndOverlap`
  (params (OverlappedComponent :type "PrimitiveComponent Object Reference") (OtherActor :type "Actor Object Reference") (OtherComp :type "PrimitiveComponent Object Reference") (OtherBodyIndex :type Integer))
  (cast `/Game/ThirdPerson/Blueprints/BP_Sprite` OtherActor)
  (if (`self.Can Interact`)
    (bind _interactionwidget (`self.InteractionWidget`)
      (:`then`
        (if (`self.HintVisible`)
          (`UserWidget.PlayAnimation` _interactionwidget (`/Game/Blueprints/Dialogue_Interact/UI_Interact.PopUp` _interactionwidget) 0.0 1 "Forward" 1.5 false)
          (set `self.HintVisible` false)
          (set `self.CanPressE` false)
          (`MeshComponent.SetOverlayMaterial` (`self.StaticMesh`) null))
        (`KismetSystemLibrary.Delay` 0.15)
        (`Widget.RemoveFromParent` (`self.InteractionWidget`))
        (set `self.InteractionWidget` null)
        (`SceneComponent.SetVisibility` (`self.Widget`) false false))
      (:`else`))))

(fn `UserConstructionScript`)